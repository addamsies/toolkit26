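; BP_TargetBase is a target actor that hides itself and disables collision when its HitBox is overlapped, and reverses this through a Respawn event.
; A hit passes TimesToAdd and the target's construction-script Guid to BP_GameInstance.
; It then rolls against Percentage to briefly show a WBP_Barks dialogue from DT_Barks.
; The overlapping actor is destroyed, after the row's delay if a bark plays.
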(event OnComponentBeginOverlap(HitBox)
  (params (OverlappedComponent :type Primitive%20Component%20Object%20Reference) (OtherActor :type Actor%20Object%20Reference) (OtherComp :type Primitive%20Component%20Object%20Reference) (OtherBodyIndex :type Integer) (bFromSweep :type Boolean) (SweepResult :type Hit%20Result%20Structure%20%28by%20ref%29))
  ;[0.15 0.15 0.15 0.5] Set timer and on call OnDestroied event
  (CallFunction|OnDestroied)
  (bind _asbp_game_instance (Utilities|Casting|CastToBP_GameInstance (Game|GetGameInstance)))
  (Default|CallOnHit _asbp_game_instance (Variables|Default|GetTimesToAdd))
  (Default|SetTargetsArray _asbp_game_instance (Variables|Default|GetGuid))
  ;[0.15 0.15 0.15 0.5] Show intro dialogue widget with custom percentage
  (if (< (Math|Random|RandomInteger 101) (Variables|Default|Getpercentage))
    (bind _returnvalue (Utilities|GetDataTableRow "/Game/Assets/Dialogues/DT_Barks.DT_Barks" (Variables|Default|GetDialogueArray))
      (:then
        (bind _returnvalue_2 (UserInterface|CreateWidget "/Game/Blueprints/HUD/GamePlayHUD/WBP_Barks.WBP_Barks_C"))
        (Default|SetDialogue _returnvalue_2 (.DialogueArray (Utilities|Struct|BreakST_Barks _returnvalue)))
        (UserInterface|Viewport|AddtoViewport _returnvalue_2 0)
        (Utilities|FlowControl|Delay (.Delay (Utilities|Struct|BreakST_Barks _returnvalue)))
        (Widget|RemovefromParent _returnvalue_2))
      (:RowNotFound
        _)))
  (Actor|DestroyActor OtherActor))

(event Custom|Respawn
  ;[0.15 0.15 0.15 0.5] Respawn event
  (Collision|SetCollisionEnabled (Variables|Default|GetHitBox) "QueryAndPhysics")
  (Development|SetHiddeninGame (Variables|Default|GetStaticMesh) false false))

(event Custom|OnDestroied
  ;[0.15 0.15 0.15 0.5] Hidden event to call when the target get hitted
  (Collision|SetCollisionEnabled (Variables|Default|GetHitBox) "NoCollision")
  (Development|SetHiddeninGame (Variables|Default|GetStaticMesh) true false))

(fn ConstructionScript
  (Variables|Default|SetGuid (Guid|NewGuid)))