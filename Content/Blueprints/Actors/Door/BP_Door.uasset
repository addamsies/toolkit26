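; BP_Door is a double door actor that slides its two panels open when its Open event is called.
; The Opening timeline drives separate Right and Left alpha tracks that move RightDoor and LeftDoor toward RightDoorOpening and LeftDoorOpening.
; Each update lerps from the panel's current relative location rather than a stored start, so the motion compounds over the timeline.
; The event graph has no closing logic.
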(event Custom|Open
  (bind _rightdoor (Variables|Default|GetRightDoor))
  (bind _leftdoor (Variables|Default|GetLeftDoor))
  (bind (_direction _right _left) (Timeline|Opening Play)
    (:Update
      (Utilities|FlowControl|Sequence
        (:then_0
          (Transformation|SetRelativeLocation _rightdoor (Math|Vector|Lerp(Vector) (Variables|/Script/Engine.SceneComponent|GetRelativeLocation _rightdoor) (Variables|Default|GetRightDoorOpening) _right) false false))
        (:then_1
          (Transformation|SetRelativeLocation _leftdoor (Math|Vector|Lerp(Vector) (Variables|/Script/Engine.SceneComponent|GetRelativeLocation _leftdoor) (Variables|Default|GetLeftDoorOpening) _left) false false))))))

(fn ConstructionScript)