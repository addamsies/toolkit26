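; Gameplay game mode that handles respawning of the player and targets.
; Its Respawn event messages player character 0 through an interface, then respawns every BP_TargetBase actor whose Guid is recorded in the BP_GameInstance targets array.
; The array is cleaned once the matching targets have respawned.
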(event Custom|Respawn
  ;[0.15 0.15 0.15 0.5] Respawn player and targets event
  (Class|BPIPlayerInterface|IRespawnPlayer(Message) (Game|GetPlayerCharacter 0))
  (bind _asbp_game_instance (Utilities|Casting|CastToBP_GameInstance (Game|GetGameInstance)))
  (Variables|Default|SetAs%20BP%20Game%20Instance _asbp_game_instance)
  (bind _outactors (Actor|GetAllActorsOfClass "/Game/Blueprints/Actors/Targets/BP_TargetBase.BP_TargetBase_C"))
  (for _array_element _outactors
    (if (Utilities|Array|ContainsItem (Variables|/Game/Blueprints/GameInstance/BP_GameInstance.BP_GameInstance_C|GetTargetsArray (Variables|Default|GetAs%20BP%20Game%20Instance)) (Variables|/Game/Blueprints/Actors/Targets/BP_TargetBase.BP_TargetBase_C|GetGuid _array_element))
      (Default|Respawn _array_element)))
  (Default|CleanTargetsArray (Variables|Default|GetAs%20BP%20Game%20Instance)))

(fn ConstructionScript)